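; Spline-holding curve actor for the runtime spline editor that can append points, clear itself and convert to and from Data Table rows.
; Loading rebuilds points from scaled row positions offset by actor location, leaving stored tangents and rotations unapplied and never triggering a spline update.
; Saving writes local-space position, tangents and rotation to index-named "vert" rows.
; A getter returns world-space point structs with scaled positions.
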(fn ConstructionScript)

(fn LoadSplinefromDataTable
  (params (DataTableToLoad :type Data%20Table%20Object%20Reference) (Scale :type Float%20%28single-precision%29))
  (LocalVariables|SetSceneScale Scale)
  (Spline|ClearSplinePoints (Variables|Default|GetSpline) false)
  (bind _outrownames (DataTable|GetDataTableRowNames DataTableToLoad))
  (for _index (range 0 (Utilities|Array|LastIndex _outrownames))
    (Spline|AddSplinePoint (Variables|Default|GetSpline) (Math|Vector|MakeVector 0.0 0.0 0.0) "World" false))
  (for _index_2 (range 0 (Utilities|Array|LastIndex _outrownames))
    (bind _returnvalue (Utilities|GetDataTableRow DataTableToLoad (Utilities|Array|Get(acopy) _outrownames _index_2))
      (:then
        (Spline|SetLocationatSplinePoint (Variables|Default|GetSpline) _index_2 (+ (Math|Vector|MakeVector (* (LocalVariables|GetSceneScale) (.XPos (Utilities|Struct|BreakSplineStruct _returnvalue))) (* (LocalVariables|GetSceneScale) (.YPos (Utilities|Struct|BreakSplineStruct _returnvalue))) (* (LocalVariables|GetSceneScale) (.ZPos (Utilities|Struct|BreakSplineStruct _returnvalue)))) (Transformation|GetActorLocation)) "World" false)))))

(fn SaveSplinetoDataTable
  (params (DataTable :type Data%20Table%20Object%20Reference))
  (bind _spline (Variables|Default|GetSpline))
  ;[1 1 1] Loop through all points on spline
  (for _index (range 0 (Spline|GetNumberOfSplinePoints _spline))
    (Class|DataTableSaveFunctionLibrary|SaveDataTableRowfromName DataTable (Utilities|String|StringToName (Utilities|String|Append "vert" (Utilities|String|ToString(Integer) _index))) (Utilities|Struct|MakeSplineStruct (.X (Math|Vector|BreakVector (Spline|GetLocationatSplinePoint _spline _index "Local"))) (.Y (Math|Vector|BreakVector (Spline|GetLocationatSplinePoint _spline _index "Local"))) (.Z (Math|Vector|BreakVector (Spline|GetLocationatSplinePoint _spline _index "Local"))) (.X (Math|Vector|BreakVector (Spline|GetArriveTangentatSplinePoint _spline _index "Local"))) (.Y (Math|Vector|BreakVector (Spline|GetArriveTangentatSplinePoint _spline _index "Local"))) (.Z (Math|Vector|BreakVector (Spline|GetArriveTangentatSplinePoint _spline _index "Local"))) (.X (Math|Vector|BreakVector (Spline|GetLeaveTangentatSplinePoint _spline _index "Local"))) (.Y (Math|Vector|BreakVector (Spline|GetLeaveTangentatSplinePoint _spline _index "Local"))) (.Z (Math|Vector|BreakVector (Spline|GetLeaveTangentatSplinePoint _spline _index "Local"))) (.Roll (Math|Rotator|BreakRotator (Spline|GetRotationatSplinePoint _spline _index "Local"))) (.Pitch (Math|Rotator|BreakRotator (Spline|GetRotationatSplinePoint _spline _index "Local"))) (.Yaw (Math|Rotator|BreakRotator (Spline|GetRotationatSplinePoint _spline _index "Local")))))))

(fn GetAllSplinePoints
  (params (Scale :type Float%20%28single-precision%29))
  (bind _spline (Variables|Default|GetSpline))
  ;[1 1 1] Loop through all points on spline
  (for _index (range 0 (Spline|GetNumberOfSplinePoints _spline))
    (Utilities|Array|Add (LocalVariables|GetSplineP) (Utilities|Struct|MakeSplineStruct (* Scale (.X (Math|Vector|BreakVector (Spline|GetLocationatSplinePoint _spline _index "World")))) (* Scale (.Y (Math|Vector|BreakVector (Spline|GetLocationatSplinePoint _spline _index "World")))) (* Scale (.Z (Math|Vector|BreakVector (Spline|GetLocationatSplinePoint _spline _index "World")))) (.X (Math|Vector|BreakVector (Spline|GetArriveTangentatSplinePoint _spline _index "World"))) (.Y (Math|Vector|BreakVector (Spline|GetArriveTangentatSplinePoint _spline _index "World"))) (.Z (Math|Vector|BreakVector (Spline|GetArriveTangentatSplinePoint _spline _index "World"))) (.X (Math|Vector|BreakVector (Spline|GetLeaveTangentatSplinePoint _spline _index "World"))) (.Y (Math|Vector|BreakVector (Spline|GetLeaveTangentatSplinePoint _spline _index "World"))) (.Z (Math|Vector|BreakVector (Spline|GetLeaveTangentatSplinePoint _spline _index "World"))))))
  ;[1 1 1] Get the location and tangent for the current point on the spline, spline point represents a keyframe
  (return (LocalVariables|GetSplineP)))

(fn AddNewSplinePoint
  (params (Position :type Vector%20%28by%20ref%29))
  (Spline|AddSplinePointatIndex (Variables|Default|GetSpline) Position (Spline|GetNumberOfSplinePoints (Variables|Default|GetSpline)) "World" true))

(fn ClearSpline
  (Spline|ClearSplinePoints (Variables|Default|GetSpline) true))