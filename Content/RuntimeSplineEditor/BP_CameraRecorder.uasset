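; Camera recorder actor that records keyframes as spline points and flies itself along saved camera paths.
; On BeginPlay it loads a data table into the first BP_CurveObject found and caches the points; Tick lerps through them in a loop.
; The S key and BPI events add points at its current location, but time and focus go unused.
; Timeline playback and saving exist but are never triggered here.
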(event Custom|PlayCurveOnTimeline
  (Variables|Default|SetStartPosition (Transformation|GetActorLocation))
  ;[1 1 1] Set Camera Object Position and rotation from curve
  (bind (_direction _cameraposition _camerarotation _xposition) (Timeline|PlayCameraAnimation Play)
    (:Update
      (Transformation|SetActorLocation (Math|Vector|MakeVector _xposition 0.0 0.0) false false)
      (Transformation|SetActorRotation (Math|Rotator|MakeRotator (.X (Math|Vector|BreakVector _camerarotation)) (.Y (Math|Vector|BreakVector _camerarotation)) (.Z (Math|Vector|BreakVector _camerarotation)))))))

(event Custom|AnimateUsingWaypoints
  (if (> (Utilities|Array|Length (Variables|Default|GetCameraAnimationKeys)) 0)
    ;[1 1 1] Set Camera location over time, based on position of curve
    (Transformation|SetActorLocation (Math|Vector|Lerp(Vector) (Transformation|GetActorLocation) (Math|Vector|MakeVector (.XPos (Utilities|Struct|BreakSplineStruct (Utilities|Array|Get(acopy) (Variables|Default|GetCameraAnimationKeys) (Variables|Default|GetNextGoalCurve)))) (.YPos (Utilities|Struct|BreakSplineStruct (Utilities|Array|Get(acopy) (Variables|Default|GetCameraAnimationKeys) (Variables|Default|GetNextGoalCurve)))) (.ZPos (Utilities|Struct|BreakSplineStruct (Utilities|Array|Get(acopy) (Variables|Default|GetCameraAnimationKeys) (Variables|Default|GetNextGoalCurve))))) 0.1) false false)
    ;[1 1 1] If we have reached close proximity of goal location
    (if (< (Math|Vector|Distance(Vector) (Transformation|GetActorLocation) (Math|Vector|MakeVector (.XPos (Utilities|Struct|BreakSplineStruct (Utilities|Array|Get(acopy) (Variables|Default|GetCameraAnimationKeys) (Variables|Default|GetNextGoalCurve)))) (.YPos (Utilities|Struct|BreakSplineStruct (Utilities|Array|Get(acopy) (Variables|Default|GetCameraAnimationKeys) (Variables|Default|GetNextGoalCurve)))) (.ZPos (Utilities|Struct|BreakSplineStruct (Utilities|Array|Get(acopy) (Variables|Default|GetCameraAnimationKeys) (Variables|Default|GetNextGoalCurve)))))) 25.0)
      ;[1 1 1] Go to next keyframe or go back to start
      (Math|Integer|IncrementInt (Variables|Default|GetNextGoalCurve)
        (:%20%20
          (if (>= (Variables|Default|GetNextGoalCurve) (Utilities|Array|Length (Variables|Default|GetCameraAnimationKeys)))
            (Variables|Default|SetNextGoalCurve 0)))))))

(event EventBeginPlay
  (CallFunction|LoadSplinefromDataTable)
  (bind _splinepointsout (CallFunction|GetAllPointsonSpline))
  (Variables|Default|SetCameraAnimationKeys _splinepointsout))

(event Collision|EventActorBeginOverlap
  (params (OtherActor :type Actor%20Object%20Reference)))

(event EventTick
  (params (DeltaSeconds :type Float%20%28single-precision%29))
  (CallFunction|AnimateUsingWaypoints))

(event EventBPIAddNewKeyframe
  (params (Time :type Float%20%28single-precision%29))
  (CallFunction|AddKeyframe Time))

(event EventBPIDeleteCameraAnimation
  (bind (_isvalid_ _splinerecorderinstance) (CallFunction|GetSplineRecorderInstance))
  ;[1 1 1] Clear Existing animation
  (if _isvalid_
    (Default|ClearSpline _splinerecorderinstance)))

(event EventBPIDeleteKeyframebyIndex
  (params (KeyIndex :type Integer))
  (if (> (Utilities|Array|Length (Variables|Default|GetCameraAnimationKeys)) KeyIndex)
    (Utilities|Array|RemoveIndex (Variables|Default|GetCameraAnimationKeys) KeyIndex)))

(event EventBPICreateNewCameraAnimation
  (params (AnimationName :type String))
  (Spline|ClearSplinePoints (Variables|Default|GetCameraTrackSpline) true)
  (Variables|Default|SetCameraAnimationName AnimationName))

(event EventBPILoadCameraAnimation)

(event Input|KeyboardEvents|S
  (params (Key :type Key%20Structure))
  (:Pressed
    (Development|PrintString "Set new keyframe")
    ;[1 1 1] What is the time from the timeline?
    (bind _currentframe (Class|BPIVertexInstance|BPIGetCurrentFrameMasterTimeline(Message) (Game|GetGameInstance)))
    (Development|PrintString (Utilities|String|ToString(Float) (Math|Conversions|ToFloat(Integer) _currentframe)))
    (CallFunction|AddKeyframe (Math|Conversions|ToFloat(Integer) _currentframe))))

(fn ConstructionScript)

(fn AddKeyframe
  (params (Time :type Float%20%28single-precision%29))
  (bind _returnvalue (Transformation|GetActorTransform))
  (bind (_isvalid_ _splinerecorderinstance) (CallFunction|GetSplineRecorderInstance))
  ;[1 1 1] This is the position of the camera to save
  (LocalVariables|SetCurrentCameraTransform _returnvalue)
  ;[1 1 1] This is where you grab the properties of the camera at this time on the timeline
  (LocalVariables|SetCurrentCameraFocusSettings (Variables|/Script/CinematicCamera.CineCameraComponent|GetFocusSettings (Variables|Default|GetCineCamera)))
  ;[1 1 1] Create a spline point based on this new location(From current position)
  (if _isvalid_
    (Default|AddNewSplinePoint _splinerecorderinstance (.Location (Math|Transform|BreakTransform _returnvalue)))))

(fn GetAllPointsonSpline
  (bind (_isvalid_ _splinerecorderinstance) (CallFunction|GetSplineRecorderInstance))
  (if _isvalid_
    (bind _splinepointsout (Default|GetAllSplinePoints _splinerecorderinstance 1.0))
    (return _splinepointsout)))

(fn SaveCameraAnimation)

(fn LoadSplinefromDataTable
  (bind (_isvalid_ _splinerecorderinstance) (CallFunction|GetSplineRecorderInstance))
  (if _isvalid_
    (Default|LoadSplinefromDataTable _splinerecorderinstance (Variables|Default|GetCameraAnimationFile) (Variables|Default|GetsceneScale))))

(fn SaveSplinetoDataTable
  (bind (_isvalid_ _splinerecorderinstance) (CallFunction|GetSplineRecorderInstance))
  (if _isvalid_
    (Default|SaveSplinetoDataTable _splinerecorderinstance (Variables|Default|GetCameraAnimationFile))))

(fn GetSplineRecorderInstance
  (bind _outactors (Actor|GetAllActorsOfClass "/Game/RuntimeSplineEditor/BP_CurveObject.BP_CurveObject_C"))
  (if (> (Utilities|Array|Length _outactors) 0)
    (return (> (Utilities|Array|Length _outactors) 0) (Utilities|Array|Get(acopy) _outactors))))

(fn BPIGetAllKeyframes
  (return (Variables|Default|GetCameraAnimationKeys)))