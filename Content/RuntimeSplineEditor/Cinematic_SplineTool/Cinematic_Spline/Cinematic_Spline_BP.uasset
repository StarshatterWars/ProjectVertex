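; Cinematic camera spline actor that plays cutscenes along a path and supports runtime editing of that path.
; While Play is set, Tick advances Speed (distance along the spline) to move an arrow with CameraActor attached.
; At the end it chains to NextCutScene or returns view and input to the player.
; Editing functions scrub and preview, add keyframes, move points via spawned RTT_Actor handles, and save/load through a data table.
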(event Custom|Update
  ;[0 0 0] Update
)

(event Custom|ManualMoveTimeline
  (params (Speed_Editor :type Float%20%28single-precision%29))
  (Variables|Default|SetSpeed Speed_Editor)
  (Utilities|LocationRotationCameraSpline))

(event EventBeginPlay
  ;[0 0 0] BeginPlay
  (Utilities|FlowControl|Sequence
    (:then_0
      (Variables|Default|SethasInitialized true)
      (Utilities|IsValid (Variables|Default|GetObject)
        (:Is%20Valid
          _)
        (:Is%20Not%20Valid
          (Variables|Default|SetObject (Game|GetPlayerCharacter 0))))
      (switch Utilities|FlowControl|Switch|SwitchonActivationTime (Variables|Default|GetActivateCamera)
        (:NewEnumerator0
          (Variables|Default|SetSpeed 0.0)
          (if (>= (Variables|Default|GetSpeed) (Spline|GetSplineLength (Variables|Default|GetSpline)))
            (Utilities|FlowControl|DoOnce false
              (:Completed
                (Variables|Default|SetSpeed (Spline|GetSplineLength (Variables|Default|GetSpline)))
                (bind _outactors (Actor|GetAllActorsOfClass "Cinematic_Spline_BP_C"))
                (for _array_element _outactors
                  (Variables|Cinematic_Spline_BP_C|SetSpeed _array_element (Spline|GetSplineLength (Variables|Cinematic_Spline_BP_C|GetSpline _array_element))))))))))
    (:then_1
      (CallFunction|CreateSelectableObjPerSplinePoint))))

(event EventTick
  (params (DeltaSeconds :type Float%20%28single-precision%29))
  (bind _returnvalue (Game|GetPlayerCharacter 0))
  (bind _actordestroy (Variables|Default|GetActorDestroy))
  (bind _nextcutscene (Variables|Default|GetNextCutScene))
  (bind _actordestroy_2 (Variables|Default|GetActorDestroy))
  ;[0 0 0] Update
  (if (Variables|Default|GethasInitialized)
    (Utilities|FlowControl|Sequence
      (:then_0
        (if (Variables|Default|GetPlay)
          (Utilities|LocationRotationCameraSpline)))
      (:then_1
        (if (>= (Variables|Default|GetSpeed) (Spline|GetSplineLength (Variables|Default|GetSpline)))
          (Utilities|FlowControl|DoOnce false :!label _label
            (:Completed
              (Utilities|IsValid (Variables|Default|GetNextCutScene)
                (:Is%20Valid
                  (Game|Player|SetViewTargetwithBlend (Game|GetPlayerController 0) (Variables|Cinematic_Spline_BP_C|GetCameraActor _nextcutscene) 0.0 "VTBlend_EaseIn" 0.0 false)
                  (Variables|Cinematic_Spline_BP_C|SetSpeed _nextcutscene 0.0)
                  (Variables|Cinematic_Spline_BP_C|SetPlay _nextcutscene true)
                  (Audio|PlaySound2D (Variables|Cinematic_Spline_BP_C|GetSFX _nextcutscene) 1.0 1.0 0.0 0 0)
                  (Utilities|IsValid _actordestroy
                    (:Is%20Valid
                      (Actor|DestroyActor _actordestroy))))
                (:Is%20Not%20Valid
                  (switch Utilities|FlowControl|Switch|SwitchonCameraSwitching (Variables|Default|GetCameraSwitching)
                    (:NewEnumerator0
                      (Game|Player|SetViewTargetwithBlend (Game|GetPlayerController 0) (Game|GetPlayerCharacter 0) 0.5 "VTBlend_EaseIn" 0.5 false))
                    (:NewEnumerator1
                      (Game|Player|SetViewTargetwithBlend (Game|GetPlayerController 0) (Game|GetPlayerCharacter 0) 0.0 "VTBlend_EaseIn" 0.0 false)))
                  (Utilities|IsValid _returnvalue
                    (:Is%20Valid
                      (Input|EnableInput _returnvalue (Game|GetPlayerController 0))
                      (Utilities|IsValid _actordestroy_2
                        (:Is%20Valid
                          (Actor|DestroyActor _actordestroy_2)))))))))
          (else
            (goto _label Reset)))))))

(fn ConstructionScript
  (bind _spline (Variables|Default|GetSpline))
  (if (Variables|Default|GetClosedSpline)
    (Spline|SetClosedLoop _spline true true)
    (else
      (Spline|SetClosedLoop _spline false true)))
  (switch Utilities|FlowControl|Switch|SwitchonActivationTime (Variables|Default|GetActivateCamera)
    (:NewEnumerator0
      (Utilities|FlowControl|DoOnce false :!label _label
        (:Completed
          (bind _outactors (Actor|GetAllActorsOfClass "Cinematic_Spline_BP_C"))
          (for _array_element _outactors
            (if (!= _array_element self)
              (Utilities|IsValid _array_element
                (:Is%20Valid
                  (switch Utilities|FlowControl|Switch|SwitchonActivationTime (Variables|Cinematic_Spline_BP_C|GetActivateCamera _array_element)
                    (:NewEnumerator0
                      (Variables|Cinematic_Spline_BP_C|SetActivateCamera _array_element "NewEnumerator1"))
                    (:NewEnumerator1
                      (Variables|Cinematic_Spline_BP_C|SetActivateCamera _array_element "NewEnumerator1"))
                    (:NewEnumerator2
                      (Variables|Cinematic_Spline_BP_C|SetActivateCamera _array_element "NewEnumerator2"))))))))))
    (:NewEnumerator1
      (goto _label Reset))))

(fn SaveSpline
  (CallFunction|SaveSplinetoDataTable (Variables|Default|GetSpline) (Variables|Default|GetCameraAnimation)))

(fn LoadSpline
  (CallFunction|LoadSplinefromDataTable (Variables|Default|GetSpline) 1.0 (Variables|Default|GetCameraAnimation) (Transformation|GetActorLocation) (Transformation|GetActorRotation)))

(fn SetCameraonTimeline
  (params (Time :type Float%20%28single-precision%29))
  (CallFunction|ManualMoveTimeline Time))

(fn AddKeyframe
  (bind _splineidx (CallFunction|GetSplineIndexbyDistance))
  (Spline|AddSplinePointatIndex (Variables|Default|GetSpline) (Transformation|GetActorLocation (Variables|Default|GetCameraActor)) _splineidx "World" true))

(fn GetSplineIndexbySpeed
  (bind _index (Utilities|FlowControl|ForLoopwithBreak 0 (Spline|GetNumberOfSplinePoints (Variables|Default|GetSpline)) :!label _label)
    (:LoopBody
      (LocalVariables|SetfoundLoc _index)
      (if (> (Spline|GetDistanceAlongSplineatSplinePoint (Variables|Default|GetSpline) _index) (Variables|Default|GetSpeed))
        (goto _label Break)))
    (:Completed
      (return (LocalVariables|GetfoundLoc)))))

(fn GetSplineIndexbyDistance
  (bind _spline (Variables|Default|GetSpline))
  (bind _index (Utilities|FlowControl|ForLoopwithBreak 0 (Spline|GetNumberOfSplinePoints _spline))
    (:LoopBody
      (if (< (Math|Vector|Distance(Vector) (Transformation|GetActorLocation (Variables|Default|GetCameraActor)) (Spline|GetLocationatSplinePoint _spline _index "World")) (LocalVariables|GetclosestDistance))
        (LocalVariables|SetclosestDistance (Math|Vector|Distance(Vector) (Transformation|GetActorLocation (Variables|Default|GetCameraActor)) (Spline|GetLocationatSplinePoint _spline _index "World")))
        (LocalVariables|SetfoundLoc _index)))
    (:Completed
      (return (LocalVariables|GetfoundLoc)))))

(fn SetCameraonTimelinebyMinMaxTime
  (params (CurrentTimeOnSegment :type Float%20%28single-precision%29) (MaxSegmentTime :type Float%20%28single-precision%29))
  ;[1 1 1] Stop Playback
  (Variables|Default|SetPlay false)
  ;[1 1 1] Avoid divide by 0
  (if (> CurrentTimeOnSegment 0.0)
    (CallFunction|SetCameraonTimeline (* (Spline|GetSplineLength (Variables|Default|GetSpline)) (/ CurrentTimeOnSegment MaxSegmentTime)))
    (else
      (CallFunction|SetCameraonTimeline 0.0))))

(fn PreviewCameraView
  (Game|Player|SetViewTargetwithBlend (Game|GetPlayerController 0) (Variables|Default|GetCameraActor) 0.25 "VTBlend_Linear" 0.0 false))

(fn AddAdditionalKeyframe
  (Spline|AddSplinePointatIndex (Variables|Default|GetSpline) (Transformation|GetActorLocation (Variables|Default|GetCameraActor)) (Spline|GetNumberOfSplinePoints (Variables|Default|GetSpline)) "World" true))

(fn CreateSelectableObjPerSplinePoint
  (bind _spline (Variables|Default|GetSpline))
  (for _index (range 0 (Spline|GetNumberOfSplinePoints _spline))
    (bind _returnvalue (Game|SpawnActorfromClass "/Game/RuntimeSplineEditor/RTT_Shared/RTT_Actor.RTT_Actor_C" (Math|Transform|MakeTransform (Spline|GetLocationatSplinePoint _spline _index "World") (Spline|GetRotationatSplinePoint _spline _index "Local") "0.020000,0.020000,0.020000") "AlwaysSpawn" 0 _index self 0))
    (Variables|/Game/RuntimeSplineEditor/RTT_Shared/RTT_Actor.RTT_Actor_C|SetsplineID _returnvalue _index)))

(fn RemoveSelectableObjbySplinePoint
  (params (SplinePointIdx :type Integer))
  (if (> (Spline|GetNumberOfSplinePoints (Variables|Default|GetSpline)) SplinePointIdx)
    _))

(fn SetSplinePointTransform
  (params (PointTransform :type Transform) (PointIndex :type Integer) (isTangentIn :type Boolean) (isTangentOut :type Boolean))
  (bind (_location _rotation) (Math|Transform|BreakTransform PointTransform))
  (bind _spline (Variables|Default|GetSpline))
  (LocalVariables|SettangentsIn (Spline|GetArriveTangentatSplinePoint _spline PointIndex "Local"))
  (LocalVariables|SettangentsOut (Spline|GetLeaveTangentatSplinePoint _spline PointIndex "Local"))
  (if (> (Spline|GetNumberOfSplinePoints _spline) PointIndex)
    (Spline|SetLocationatSplinePoint _spline PointIndex _location "World" false)
    (Spline|SetRotationatSplinePoint _spline PointIndex _rotation "World" false)
    (Spline|SetTangentsatSplinePoint _spline PointIndex (LocalVariables|GettangentsIn) (LocalVariables|GettangentsOut) "Local" true)))