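; Spline actor that converts a camera curve between a spline component and the CameraCurve data table.
; Loading rebuilds points from table rows as positions offset by actor location; tangent restore is unwired and spline updates are suppressed.
; Saving writes local positions and world-space tangents to index-named rows, and GetAllSplinePoints returns the same structs as an array.
; The event graph triggers nothing.
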(event EventBeginPlay)

(event Collision|EventActorBeginOverlap
  (params (OtherActor :type Actor%20Object%20Reference)))

(event EventTick
  (params (DeltaSeconds :type Float%20%28single-precision%29)))

(fn ConstructionScript)

(fn LoadSplinefromDataTable
  (Spline|ClearSplinePoints (Variables|Default|GetSpline) false)
  (bind _outrownames (DataTable|GetDataTableRowNames (Variables|Default|GetCameraCurve)))
  (for _index (range 0 (Utilities|Array|LastIndex _outrownames))
    (Spline|AddSplinePoint (Variables|Default|GetSpline) (Math|Vector|MakeVector 0.0 0.0 0.0) "World" false))
  (for _index_2 (range 0 (Utilities|Array|LastIndex _outrownames))
    (bind _returnvalue (Utilities|GetDataTableRow (Variables|Default|GetCameraCurve) (Utilities|Array|Get(acopy) _outrownames _index_2))
      (:then
        (Spline|SetLocationatSplinePoint (Variables|Default|GetSpline) _index_2 (+ (Math|Vector|MakeVector (.XPos (Utilities|Struct|BreakSplineStruct _returnvalue)) (.YPos (Utilities|Struct|BreakSplineStruct _returnvalue)) (.ZPos (Utilities|Struct|BreakSplineStruct _returnvalue))) (Transformation|GetActorLocation)) "World" false)))))

(fn SaveSplinetoFile
  (bind _spline (Variables|Default|GetSpline))
  ;[1 1 1] Loop through all points on spline
  (for _index (range 0 (Spline|GetNumberOfSplinePoints _spline))
    (Class|DataTableSaveFunctionLibrary|SaveDataTableRowfromName (Variables|Default|GetCameraCurve) (Utilities|String|StringToName (Utilities|String|Append "vert" (Utilities|String|ToString(Integer) _index))) (Utilities|Struct|MakeSplineStruct (.X (Math|Vector|BreakVector (Spline|GetLocationatSplinePoint _spline _index "Local"))) (.Y (Math|Vector|BreakVector (Spline|GetLocationatSplinePoint _spline _index "Local"))) (.Z (Math|Vector|BreakVector (Spline|GetLocationatSplinePoint _spline _index "Local"))) (.X (Math|Vector|BreakVector (Spline|GetArriveTangentatSplinePoint _spline _index "World"))) (.Y (Math|Vector|BreakVector (Spline|GetArriveTangentatSplinePoint _spline _index "World"))) (.Z (Math|Vector|BreakVector (Spline|GetArriveTangentatSplinePoint _spline _index "World"))) (.X (Math|Vector|BreakVector (Spline|GetLeaveTangentatSplinePoint _spline _index "World"))) (.Y (Math|Vector|BreakVector (Spline|GetLeaveTangentatSplinePoint _spline _index "World"))) (.Z (Math|Vector|BreakVector (Spline|GetLeaveTangentatSplinePoint _spline _index "World")))))))

(fn GetAllSplinePoints
  (bind _spline (Variables|Default|GetSpline))
  ;[1 1 1] Loop through all points on spline
  (for _index (range 0 (Spline|GetNumberOfSplinePoints _spline))
    (Utilities|Array|Add (LocalVariables|GetSplinePoints) (Utilities|Struct|MakeSplineStruct (.X (Math|Vector|BreakVector (Spline|GetLocationatSplinePoint _spline _index "Local"))) (.Y (Math|Vector|BreakVector (Spline|GetLocationatSplinePoint _spline _index "Local"))) (.Z (Math|Vector|BreakVector (Spline|GetLocationatSplinePoint _spline _index "Local"))) (.X (Math|Vector|BreakVector (Spline|GetArriveTangentatSplinePoint _spline _index "World"))) (.Y (Math|Vector|BreakVector (Spline|GetArriveTangentatSplinePoint _spline _index "World"))) (.Z (Math|Vector|BreakVector (Spline|GetArriveTangentatSplinePoint _spline _index "World"))) (.X (Math|Vector|BreakVector (Spline|GetLeaveTangentatSplinePoint _spline _index "World"))) (.Y (Math|Vector|BreakVector (Spline|GetLeaveTangentatSplinePoint _spline _index "World"))) (.Z (Math|Vector|BreakVector (Spline|GetLeaveTangentatSplinePoint _spline _index "World"))))))
  ;[1 1 1] Get the location and tangent for the current point on the spline, spline point represents a keyframe
  (return (LocalVariables|GetSplinePoints)))