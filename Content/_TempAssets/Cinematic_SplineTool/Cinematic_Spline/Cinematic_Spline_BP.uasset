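; Cinematic spline camera tool that plays in-game cutscenes by moving a camera actor along an editable spline.
; Playback starts on BeginPlay or box overlap, switches the view target and disables player input, while a looping timer advances spline distance.
; At the end it chains to NextCutScene or returns view and input to the player.
; Helper functions scrub the timeline, add keyframes and save or load the spline through a DataTable.
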(event OnComponentBeginOverlap(Box)
  (params (OverlappedComponent :type Primitive%20Component%20Object%20Reference) (OtherActor :type Actor%20Object%20Reference) (OtherComp :type Primitive%20Component%20Object%20Reference) (OtherBodyIndex :type Integer) (bFromSweep :type Boolean) (SweepResult :type Hit%20Result%20Structure%20%28by%20ref%29))
  (bind _object (Variables|Default|GetObject))
  ;[0 0 0] BoxOverLap
  (Utilities|IsValid _object
    (:Is%20Valid
      (if (== OtherActor _object)
        (Variables|Default|SetPlay true)
        (switch Utilities|FlowControl|Switch|Switchon (Variables|Default|GetActivateCamera)
          (:NewEnumerator1
            (switch Utilities|FlowControl|Switch|Switchon (Variables|Default|GetCameraSwitching)
              (:NewEnumerator0
                (switch Utilities|FlowControl|Switch|Switchon (Variables|Default|GetReplay)
                  (:NewEnumerator0
                    (Utilities|FlowControl|DoOnce false
                      (:Completed
                        (Variables|Default|SetSpeed 0.0)
                        (Game|Player|SetViewTargetwithBlend (Game|GetPlayerController 0) (Variables|Default|GetCameraActor) 0.5 "VTBlend_EaseIn" 0.5 false)
                        (Audio|PlaySound2D (Variables|Default|GetSFX) 1.0 1.0 0.0 0 0))))
                  (:NewEnumerator1
                    (Variables|Default|SetSpeed 0.0)
                    (Game|Player|SetViewTargetwithBlend (Game|GetPlayerController 0) (Variables|Default|GetCameraActor) 0.5 "VTBlend_EaseIn" 0.5 false)
                    (Audio|PlaySound2D (Variables|Default|GetSFX) 1.0 1.0 0.0 0 0)))
                (Input|DisableInput (Game|GetPlayerCharacter 0) (Game|GetPlayerController 0))
                (if (>= (Variables|Default|GetSpeed) (Spline|GetSplineLength (Variables|Default|GetSpline)))
                  (Collision|SetCollisionEnabled (Variables|Default|GetBox) "NoCollision")
                  (Variables|Default|SetPlay false)))
              (:NewEnumerator1
                (switch Utilities|FlowControl|Switch|Switchon (Variables|Default|GetReplay)
                  (:NewEnumerator0
                    (Utilities|FlowControl|DoOnce false
                      (:Completed
                        (Variables|Default|SetSpeed 0.0)
                        (Game|Player|SetViewTargetwithBlend (Game|GetPlayerController 0) (Variables|Default|GetCameraActor) 0.0 "VTBlend_Linear" 0.0 false)
                        (Audio|PlaySound2D (Variables|Default|GetSFX) 1.0 1.0 0.0 0 0))))
                  (:NewEnumerator1
                    (Variables|Default|SetSpeed 0.0)
                    (Game|Player|SetViewTargetwithBlend (Game|GetPlayerController 0) (Variables|Default|GetCameraActor) 0.0 "VTBlend_Linear" 0.0 false)
                    (Audio|PlaySound2D (Variables|Default|GetSFX) 1.0 1.0 0.0 0 0)))
                (Input|DisableInput (Game|GetPlayerCharacter 0) (Game|GetPlayerController 0))
                (if (>= (Variables|Default|GetSpeed) (Spline|GetSplineLength (Variables|Default|GetSpline)))
                  (Collision|SetCollisionEnabled (Variables|Default|GetBox) "NoCollision")
                  (Variables|Default|SetPlay false))))))))))

(event Custom|Update
  (bind _returnvalue (Game|GetPlayerCharacter 0))
  (bind _actordestroy (Variables|Default|GetActorDestroy))
  (bind _nextcutscene (Variables|Default|GetNextCutScene))
  (bind _actordestroy_2 (Variables|Default|GetActorDestroy))
  ;[0 0 0] Update
  (Utilities|FlowControl|Sequence
    (:then_0
      (if (Variables|Default|GetPlay)
        (Utilities|LocationRotationCameraSpline)))
    (:then_1
      (if (>= (Variables|Default|GetSpeed) (Spline|GetSplineLength (Variables|Default|GetSpline)))
        (Utilities|FlowControl|DoOnce false :!label _label
          (:Completed
            (Utilities|IsValid (Variables|Default|GetNextCutScene)
              (:Is%20Valid
                (Game|Player|SetViewTargetwithBlend (Game|GetPlayerController 0) (Variables|Cinematic_Spline_BP_C|GetCameraActor _nextcutscene) 0.0 "VTBlend_EaseIn" 0.0 false)
                (Variables|Cinematic_Spline_BP_C|SetSpeed _nextcutscene 0.0)
                (Variables|Cinematic_Spline_BP_C|SetPlay _nextcutscene true)
                (Audio|PlaySound2D (Variables|Cinematic_Spline_BP_C|GetSFX _nextcutscene) 1.0 1.0 0.0 0 0)
                (Utilities|IsValid _actordestroy
                  (:Is%20Valid
                    (Actor|DestroyActor _actordestroy))))
              (:Is%20Not%20Valid
                (switch Utilities|FlowControl|Switch|Switchon (Variables|Default|GetCameraSwitching)
                  (:NewEnumerator0
                    (Game|Player|SetViewTargetwithBlend (Game|GetPlayerController 0) (Game|GetPlayerCharacter 0) 0.5 "VTBlend_EaseIn" 0.5 false))
                  (:NewEnumerator1
                    (Game|Player|SetViewTargetwithBlend (Game|GetPlayerController 0) (Game|GetPlayerCharacter 0) 0.0 "VTBlend_EaseIn" 0.0 false)))
                (Utilities|IsValid _returnvalue
                  (:Is%20Valid
                    (Input|EnableInput _returnvalue (Game|GetPlayerController 0))
                    (Utilities|IsValid _actordestroy_2
                      (:Is%20Valid
                        (Actor|DestroyActor _actordestroy_2)))))))))
        (else
          (goto _label Reset))))))

(event Custom|ManualMoveTimeline
  (params (Speed_Editor :type Float%20%28single-precision%29))
  (Variables|Default|SetSpeed Speed_Editor)
  (Utilities|LocationRotationCameraSpline))

(event EventBeginPlay
  (bind _returnvalue (Game|GetPlayerController 0))
  (bind _returnvalue_2 (Game|GetPlayerCharacter 0))
  ;[0 0 0] BeginPlay
  (Utilities|FlowControl|Sequence
    (:then_0
      (bind _asvertex_instance (Utilities|Casting|CastToVertexInstance (Game|GetGameInstance)))
      (Variables|Default|SetAs%20Vertex%20Instance _asvertex_instance))
    (:then_1
      (Utilities|Time|SetTimerbyFunctionName 0 "Update" 0.03 true)
      (Utilities|IsValid (Variables|Default|GetObject)
        (:Is%20Valid
          _)
        (:Is%20Not%20Valid
          (Variables|Default|SetObject (Game|GetPlayerCharacter 0))))
      (switch Utilities|FlowControl|Switch|Switchon (Variables|Default|GetActivateCamera)
        (:NewEnumerator0
          (Variables|Default|SetPlay true)
          (Variables|Default|SetSpeed 0.0)
          (Audio|PlaySound2D (Variables|Default|GetSFX) 1.0 1.0 0.0 0 0)
          (Game|Player|SetViewTargetwithBlend (Game|GetPlayerController 0) (Variables|Default|GetCameraActor) 0.0 "VTBlend_Linear" 0.0 false)
          (Utilities|IsValid _returnvalue
            (:Is%20Valid
              (Input|DisableInput _returnvalue_2 _returnvalue))
            (:Is%20Not%20Valid
              (Input|DisableInput _returnvalue_2 _returnvalue)))
          (if (>= (Variables|Default|GetSpeed) (Spline|GetSplineLength (Variables|Default|GetSpline)))
            (Utilities|FlowControl|DoOnce false
              (:Completed
                (Variables|Default|SetSpeed (Spline|GetSplineLength (Variables|Default|GetSpline)))
                (bind _outactors (Actor|GetAllActorsOfClass "Cinematic_Spline_BP_C"))
                (for _array_element _outactors
                  (Variables|Cinematic_Spline_BP_C|SetSpeed _array_element (Spline|GetSplineLength (Variables|Cinematic_Spline_BP_C|GetSpline _array_element))))))))))))

(event Input|KeyboardEvents|S
  (params (Key :type Key%20Structure))
  (:Pressed
    (Development|PrintString "Set Keyframe")))

(fn ConstructionScript
  (bind _spline (Variables|Default|GetSpline))
  (bind _box (Variables|Default|GetBox))
  (Components|Box|SetBoxExtent (Variables|Default|GetBox) (Variables|Default|GetBoxExtent) true)
  (Transformation|SetRelativeLocation (Variables|Default|GetBox) (Variables|Default|GetBoxLocation) false false)
  (if (Variables|Default|GetClosedSpline)
    (Spline|SetClosedLoop _spline true true)
    (else
      (Spline|SetClosedLoop _spline false true)))
  (switch Utilities|FlowControl|Switch|Switchon (Variables|Default|GetActivateCamera)
    (:NewEnumerator0
      (Rendering|SetVisibility (Variables|Default|GetBox) false false))
    (:NewEnumerator1
      (Rendering|SetVisibility _box true false))
    (:NewEnumerator2
      (Rendering|SetVisibility _box false false)))
  (switch Utilities|FlowControl|Switch|Switchon (Variables|Default|GetActivateCamera)
    (:NewEnumerator0
      (Utilities|FlowControl|DoOnce false :!label _label
        (:Completed
          (bind _outactors (Actor|GetAllActorsOfClass "Cinematic_Spline_BP_C"))
          (for _array_element _outactors
            (if (!= _array_element self)
              (Utilities|IsValid _array_element
                (:Is%20Valid
                  (switch Utilities|FlowControl|Switch|Switchon (Variables|Cinematic_Spline_BP_C|GetActivateCamera _array_element)
                    (:NewEnumerator0
                      (Variables|Cinematic_Spline_BP_C|SetActivateCamera _array_element 0)
                      (Rendering|SetVisibility (Variables|Cinematic_Spline_BP_C|GetBox _array_element) true false))
                    (:NewEnumerator1
                      (Variables|Cinematic_Spline_BP_C|SetActivateCamera _array_element 0)
                      (Rendering|SetVisibility (Variables|Cinematic_Spline_BP_C|GetBox _array_element) true false))
                    (:NewEnumerator2
                      (Variables|Cinematic_Spline_BP_C|SetActivateCamera _array_element 0)
                      (Rendering|SetVisibility (Variables|Cinematic_Spline_BP_C|GetBox _array_element) false false))))))))))
    (:NewEnumerator1
      (goto _label Reset))))

(fn SaveSpline
  (CallFunction|SaveSplinetoDataTable (Variables|Default|GetSpline) (Variables|Default|GetCameraAnimation)))

(fn LoadSpline
  (CallFunction|LoadSplinefromDataTable (Variables|Default|GetSpline) 1.0 (Variables|Default|GetCameraAnimation) (Transformation|GetActorLocation) (Transformation|GetActorRotation)))

(fn SetCameraonTimeline
  (params (Time :type Float%20%28single-precision%29))
  (CallFunction|ManualMoveTimeline Time))

(fn AddKeyframe
  (bind _splineidx (CallFunction|GetSplineIndexbyDistance))
  (Spline|AddSplinePointatIndex (Variables|Default|GetSpline) (Transformation|GetActorLocation (Variables|Default|GetCameraActor)) _splineidx "World" true))

(fn GetSplineIndexbySpeed
  (bind _index (Utilities|FlowControl|ForLoopwithBreak 0 (Spline|GetNumberOfSplinePoints (Variables|Default|GetSpline)) :!label _label)
    (:LoopBody
      (LocalVariables|SetfoundLoc _index)
      (if (> (Spline|GetDistanceAlongSplineatSplinePoint (Variables|Default|GetSpline) _index) (Variables|Default|GetSpeed))
        (goto _label Break)))
    (:Completed
      (return (LocalVariables|GetfoundLoc)))))

(fn GetSplineIndexbyDistance
  (bind _spline (Variables|Default|GetSpline))
  (bind _index (Utilities|FlowControl|ForLoopwithBreak 0 (Spline|GetNumberOfSplinePoints _spline))
    (:LoopBody
      (if (< (Math|Vector|Distance(Vector) (Transformation|GetActorLocation (Variables|Default|GetCameraActor)) (Spline|GetLocationatSplinePoint _spline _index "World")) (LocalVariables|GetclosestDistance))
        (LocalVariables|SetclosestDistance (Math|Vector|Distance(Vector) (Transformation|GetActorLocation (Variables|Default|GetCameraActor)) (Spline|GetLocationatSplinePoint _spline _index "World")))
        (LocalVariables|SetfoundLoc _index)))
    (:Completed
      (return (LocalVariables|GetfoundLoc)))))

(fn SetCameraonTimelinebyMinMaxTime
  (params (CurrentTimeOnSegment :type Float%20%28single-precision%29) (MaxSegmentTime :type Float%20%28single-precision%29))
  (bind _returnvalue (/ CurrentTimeOnSegment MaxSegmentTime))
  ;[1 1 1] Stop Playback
  (Variables|Default|SetPlay false)
  ;[1 1 1] Avoid divide by 0
  (if (> CurrentTimeOnSegment 0.0)
    ;[1 1 1] Get percentage length of the spline
    (Development|PrintString (Utilities|String|ToString(Float) _returnvalue))
    (CallFunction|SetCameraonTimeline (* (Spline|GetSplineLength (Variables|Default|GetSpline)) _returnvalue))
    (else
      (CallFunction|SetCameraonTimeline 0.0))))

(fn PreviewCameraView
  (Game|Player|SetViewTargetwithBlend (Game|GetPlayerController 0) (Variables|Default|GetCameraActor) 0.25 "VTBlend_Linear" 0.0 false))

(fn AddAdditionalKeyframe
  (Spline|AddSplinePointatIndex (Variables|Default|GetSpline) (Transformation|GetActorLocation (Variables|Default|GetCameraActor)) (Spline|GetNumberOfSplinePoints (Variables|Default|GetSpline)) "World" true))