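; Utility Blueprint for the UMG color palettes that converts a color into a hex string.
; ColorToHex converts the R, G and B channels to integers and concatenates their hex forms, ignoring alpha.
; IntToHex uses repeated division by 16, mapping remainders through ToHex and the HexTable lookup, then joining them in reverse.
; Zero returns "00", but other values below 16 yield one unpadded digit.
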(fn InttoHex
  (params (In :type Integer))
  (bind _remainders (LocalVariables|GetRemainders))
  (LocalVariables|SetDivResult In)
  (while (!= (LocalVariables|GetDivResult) 0)
    (bind _hexstring (CallFunction|ToHex (Math|Integer|%(Integer) (LocalVariables|GetDivResult) 16)))
    (Utilities|Array|Add (LocalVariables|GetRemainders) _hexstring)
    (LocalVariables|SetDivResult (/ (LocalVariables|GetDivResult) 16)))
  (if (> (Utilities|Array|Length _remainders) 0)
    (bind _arrayelement (Utilities|Array|ReverseforEachLoop _remainders)
      (:LoopBody
        (LocalVariables|SetResult (Utilities|String|Append (LocalVariables|GetResult) _arrayelement)))
      (:Completed
        (return (LocalVariables|GetResult))))
    (else
      (return "00"))))

(fn ToHex
  (params (In :type Integer))
  (if (< In 10)
    (return (Utilities|String|ToString(Integer) In))
    (else
      (return (.Value (Utilities|Map|Find (LocalVariables|GetHexTable) In))))))

(fn ColortoHex
  (params (InColor :type Color%20Structure))
  (bind (_b _g _r) (Math|Color|BreakColor InColor))
  (Utilities|FlowControl|Sequence
    (:then_0
      (bind _hexstring (CallFunction|InttoHex (Math|Conversions|ToInteger(Byte) _r)))
      (LocalVariables|SetResult (Utilities|String|Append (LocalVariables|GetResult) _hexstring)))
    (:then_1
      (bind _hexstring_2 (CallFunction|InttoHex (Math|Conversions|ToInteger(Byte) _g)))
      (LocalVariables|SetResult (Utilities|String|Append (LocalVariables|GetResult) _hexstring_2)))
    (:then_2
      (bind _hexstring_3 (CallFunction|InttoHex (Math|Conversions|ToInteger(Byte) _b)))
      (bind _output_get (LocalVariables|SetResult (Utilities|String|Append (LocalVariables|GetResult) _hexstring_3)))
      (return _output_get))))