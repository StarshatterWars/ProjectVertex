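; VertexInstance builds a 3D retail planogram from data tables and also opens the main menu and test widgets.
; Planogram data sets section count and width for spawning base units; shelf data selects shelf types, placed wherever consecutive product heights change.
; Product rows spawn wide, high and deep grids of placeables.
; String fields are chopped into numbers, and actor classes are chosen by matching display names to built or indexed names, such as UPC-based ones.
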(event Custom|GetPlaceableData
  ;[1 1 1] GetPlaceable Data
  (bind _outrownames (DataTable|GetDataTableRowNames "/Game/Data/DB_ProductData.DB_ProductData"))
  (for _array_element _outrownames
    (bind _returnvalue (Utilities|GetDataTableRow "/Game/Data/DB_ProductData.DB_ProductData" _array_element)
      (:then
        (CallFunction|BuildBlueprintName (.UPC (Utilities|Struct|BreakS_Placeable _returnvalue)))
        (Variables|Placeable|SetTotal_Product (* (.Wide (Utilities|Struct|BreakS_Placeable _returnvalue)) (.High (Utilities|Struct|BreakS_Placeable _returnvalue)) (.Deep (Utilities|Struct|BreakS_Placeable _returnvalue))))
        (Variables|Placeable|Setproduct_wide (.Wide (Utilities|Struct|BreakS_Placeable _returnvalue)))
        (Variables|Placeable|Setproduct_high (.High (Utilities|Struct|BreakS_Placeable _returnvalue)))
        (Variables|Default|Setproduct_deep (.Deep (Utilities|Struct|BreakS_Placeable _returnvalue)))
        (CallFunction|SetProductLocation (.X_SIZE (Utilities|Struct|BreakS_Placeable _returnvalue)) (.Y_SIZE (Utilities|Struct|BreakS_Placeable _returnvalue)) (.Z_SIZE (Utilities|Struct|BreakS_Placeable _returnvalue)))
        (CallFunction|SetProductOffset (.Full_width (Utilities|Struct|BreakS_Placeable _returnvalue)) (.Full_height (Utilities|Struct|BreakS_Placeable _returnvalue)) (.Full_depth (Utilities|Struct|BreakS_Placeable _returnvalue)))
        (CallFunction|SpawnPlaceablefromName)))))

(event Custom|ShowMainMenu
  (bind _returnvalue (Game|GetPlayerController 0))
  (Utilities|IsValid (Variables|Default|GetMainMenuUI)
    (:Is%20Valid
      _)
    (:Is%20Not%20Valid
      (bind _returnvalue_2 (UserInterface|CreateWidget "/Game/UI/MainMenu.MainMenu_C" _returnvalue))
      (Variables|Default|SetMainMenuUI _returnvalue_2)))
  (UserInterface|Viewport|AddtoViewport (Variables|Default|GetMainMenuUI) 0)
  (Variables|/Script/Engine.PlayerController|SetbShowMouseCursor _returnvalue true))

(event Custom|Place%20Shelves
  ;[1 1 1] Find Unique Shelves by Height
  (Variables|Shelves|Setold_height 0.0)
  (Variables|Shelves|Setshelf%20number 0)
  (bind _outrownames (DataTable|GetDataTableRowNames "/Game/Data/DB_ProductData.DB_ProductData"))
  (for _array_element _outrownames
    (bind _returnvalue (Utilities|GetDataTableRow "/Game/Data/DB_ProductData.DB_ProductData" _array_element)
      (:then
        (bind _y_output (CallFunction|SetShelfYLocation (.Y_SIZE (Utilities|Struct|BreakS_Placeable _returnvalue))))
        (bind _output_get (Variables|Shelves|Setnew%20height _y_output))
        (if (not (== _output_get (Variables|Shelves|Getold_height)))
          (bind _output_get_2 (Variables|Shelves|Setold_height (Variables|Shelves|Getnew%20height)))
          (CallFunction|SetShelfXLocation (.X_SIZE (Utilities|Struct|BreakS_Placeable _returnvalue)))
          (CallFunction|PlaceShelfatLocation _output_get_2 (Variables|Shelves|Getshelf%20number)))))))

(event Custom|GetShelfByType
  ;[1 1 1] Get Shelf Data by Type
  (bind _outrownames (DataTable|GetDataTableRowNames "/Game/Data/DB_ShelfData.DB_ShelfData"))
  (for _array_element _outrownames
    (bind _returnvalue (Utilities|GetDataTableRow "/Game/Data/DB_ShelfData.DB_ShelfData" _array_element)
      (:then
        (CallFunction|SetShelfSize (.width (Utilities|Struct|BreakS_Shelve _returnvalue)) (.height (Utilities|Struct|BreakS_Shelve _returnvalue)) (.depth (Utilities|Struct|BreakS_Shelve _returnvalue)))
        (CallFunction|SetShelfOffsetLocation (.offset (Utilities|Struct|BreakS_Shelve _returnvalue)))
        (if (== (Variables|Shelves|Getshelf_depth) 25.0)
          (Variables|Shelves|SetShelf%20Size%20Increment 1)
          (else
            (Variables|Shelves|SetShelf%20Size%20Increment 0)))
        (if (== (Variables|Base|Getsection_width) 36)
          (Variables|Shelves|Setshelf%20length%20index 0)
          (bind _output_get (Variables|Shelves|Setshelf%20index (+ (* (Variables|Shelves|Getshelf%20length%20index) 2) (Variables|Shelves|GetShelf%20Size%20Increment)) :!label _label))
          (Utilities|Array|Add (Variables|Shelves|GetNew%20Shelf%20Array) (Utilities|Array|Get(acopy) (Variables|Shelves|GetShelf%20Name) _output_get))
          (bind _output_get_2 (Variables|Shelves|Setnumber%20of%20shelves (Math|Float|Truncate (/ (Variables|Shelves|Getshelf_width) (Math|Conversions|ToFloat(Integer) (Variables|Base|Getsection_width))))))
          (Utilities|Array|Add (Variables|Shelves|GetNew%20Shelf%20Numbers%20Array) _output_get_2)
          (Utilities|Array|Add (Variables|Shelves|GetNewShelfOffsetArray) (Variables|Shelves|GetSectionShelfOffset))
          (elif (== (Variables|Base|Getsection_width) 48)
            (Variables|Shelves|Setshelf%20length%20index 1)
            (goto _label)))))))

(event Custom|Place%20Shelf%20at%20Location
  (params (Shelf%20Y%20Location :type Float%20%28single-precision%29) (Shelf%20Number :type Integer) (Shelf%20Section%20Offset :type Integer))
  ;[1 1 1] Calculate Shelf Location by Section
  (Variables|Shelves|SetShelf%20Y%20Location Shelf%20Y%20Location)
  (for (_array_element _array_index) (Variables|Shelves|GetNew%20Shelf%20Array)
    (Variables|Shelves|SetShelf%20Element _array_element)
    (if (== _array_index Shelf%20Number)
      (Variables|Shelves|Setshelf%20number (+ (Variables|Shelves|Getshelf%20number) 1))
      (for (_array_element_2 _array_index_2) (Variables|Shelves|GetNew%20Shelf%20Numbers%20Array)
        (if (== Shelf%20Number _array_index_2)
          (Variables|Shelves|Settemp_shelf_section_nr _array_element_2)
          (Variables|Default|SettmpShelfOfffset (Utilities|Array|Get(acopy) (Variables|Shelves|GetNewShelfOffsetArray) _array_index_2))
          (bind _result (Math|Integer|DecrementInt (Variables|Shelves|Gettemp_shelf_section_nr))
            (:%20%20
              (for _index (range 0 _result)
                (Variables|Shelves|SetShelf%20Location (Math|Vector|MakeVector (Math|Conversions|ToFloat(Integer) (+ (* (Variables|Base|Getsection_width) _index) (* (Variables|Default|GettmpShelfOfffset) (Variables|Base|Getsection_width)))) 0.0 (- (Variables|Shelves|GetShelf%20Y%20Location) 5.0)))
                (CallFunction|SpawnShelffromName)))))))))

(event Custom|SpawnShelfFromName
  ;[1 1 1] Spawn Shelf Elementy By Name
  (for _array_element (Variables|Shelves|GetShelfElementArray)
    (bind _output_get (Variables|Shelves|SetShelfElementActor _array_element))
    (if (Utilities|Enum|Equal(Enum) (Utilities|String|LeftChop (Utilities|GetClassDisplayName _array_element) 2) (Variables|Shelves|GetShelf%20Element))
      (CallFunction|SpawnShelfElement (Utilities|GetClassDisplayName _output_get) (Variables|Shelves|GetShelf%20Location) _array_element))))

(event Custom|SpawnShelfElement
  (params (Name :type String) (Location :type Vector) (ShelfActor :type Actor%20Class%20Reference))
  ;[1 1 1] Spawn Shelf Element Actor
  (Game|SpawnActorfromClass ShelfActor (Math|Transform|MakeTransform Location) "Undefined" 0 0))

(event Custom|ShowTestUI
  ;[1 1 1] Add TestUI
  (Utilities|IsValid (Variables|Default|GetTestUI)
    (:Is%20Valid
      _)
    (:Is%20Not%20Valid
      (bind _returnvalue (UserInterface|CreateWidget "/Game/UI/TestUI.TestUI_C" (Game|GetPlayerController 0)))
      (Variables|Default|SetTestUI _returnvalue)))
  (UserInterface|Viewport|AddtoViewport (Variables|Default|GetTestUI) 0))

(event Custom|SpawnPlaceableFromName
  ;[1 1 1] Spawn Placeable from Name
  (for _array_element (Variables|Placeable|GetPlaceable)
    (Variables|Default|SetPlaceableElement _array_element)
    (if (Utilities|Enum|Equal(Enum) (Utilities|String|LeftChop (Utilities|GetClassDisplayName _array_element) 2) (Variables|Placeable|GetBA_String))
      (for _index (range 0 (- (Variables|Default|Getproduct_deep) 1))
        (for _index_2 (range 0 (- (Variables|Placeable|Getproduct_wide) 1))
          (for _index_3 (range 0 (- (Variables|Placeable|Getproduct_high) 1))
            (CallFunction|SpawnPlaceableElement (Variables|Placeable|Getplaceable_location) (Variables|Default|GetPlaceableElement) (* _index_2 (Variables|Placeable|Getx_offset)) (* _index_3 (Variables|Placeable|Gety_offset)) (* _index (Variables|Placeable|Getz_offset)))))))))

(event Custom|GetPlanogramBaseData
  ;[1 1 1] Get Planogram Base
  (bind _outrownames (DataTable|GetDataTableRowNames "/Game/Data/DB_Planogram.DB_Planogram"))
  (for _array_element _outrownames
    (bind _returnvalue (Utilities|GetDataTableRow "/Game/Data/DB_Planogram.DB_Planogram" _array_element)
      (:then
        (Variables|Base|Settotal_width (* (Math|Conversions|ToInteger(Byte) (Utilities|String|RightChop (Utilities|String|LeftChop (.Width (Utilities|Struct|BreakS_ShelfUnit _returnvalue)) 2) 6)) 12))
        (Variables|Base|SetShelveSections (Math|Conversions|ToInteger(Byte) (Utilities|String|RightChop (.Segments (Utilities|Struct|BreakS_ShelfUnit _returnvalue)) 10)))
        (Variables|Base|Setsection_width (/ (Variables|Base|Gettotal_width) (Variables|Base|GetShelveSections)))
        (if (== (Variables|Base|Getsection_width) 36)
          (Variables|Base|SetbaseIndex 0)
          (for (_array_element_2 _array_index) (Variables|Base|Getbase_name) :!label _label
            (Math|Integer|CompareInt (Variables|Base|GetbaseIndex) _array_index
              (:==
                (Variables|Base|SetbaseUnit _array_element_2)
                (Variables|Base|Setsection_offset (Variables|Base|Getsection_width))
                (CallFunction|SpawnBasefromName))))
          (elif (== (Variables|Base|Getsection_width) 48)
            (Variables|Base|SetbaseIndex 1)
            (goto _label)))))))

(event Custom|SpawnPlaceableElement
  (params (Location :type Vector) (Placeable :type Actor%20Class%20Reference) (x_offset :type Float%20%28single-precision%29) (y_offset :type Float%20%28single-precision%29) (z_offset :type Float%20%28single-precision%29))
  ;[1 1 1] Make Placeable
  (Game|SpawnActorfromClass Placeable (Math|Transform|MakeTransform (+ Location (Math|Vector|MakeVector x_offset z_offset y_offset))) "Undefined" 0 0))

(event Custom|GetShelfData
  ;[1 1 1] Get Shelf Data/ Calculate Max Shelf Depth
  (Variables|Default|Setmax_depth 0)
  (bind _outrownames (DataTable|GetDataTableRowNames "/Game/Data/DB_ShelfData.DB_ShelfData"))
  (for _array_element _outrownames
    (bind _returnvalue (Utilities|GetDataTableRow "/Game/Data/DB_ShelfData.DB_ShelfData" _array_element)
      (:then
        (bind _value (CallFunction|ShelfConverttoFloat (.height (Utilities|Struct|BreakS_Shelve _returnvalue))))
        (Variables|Shelves|Setshelf_height _value)
        (bind _value_2 (CallFunction|ShelfConverttoFloat (.width (Utilities|Struct|BreakS_Shelve _returnvalue))))
        (Variables|Shelves|Setshelf_width _value_2)
        (bind _value_3 (CallFunction|ShelfConverttoFloat (.depth (Utilities|Struct|BreakS_Shelve _returnvalue))))
        (bind _output_get (Variables|Shelves|Setshelf_depth _value_3))
        (Math|Integer|CompareInt (Math|Float|Truncate _output_get) (Variables|Default|Getmax_depth)
          (:>
            (Variables|Default|Setmax_depth (Math|Float|Truncate (Variables|Shelves|Getshelf_depth)))))))))

(event Custom|SpawnBaseFromName
  (bind _baseunit (Variables|Base|GetbaseUnit))
  ;[1 1 1] Spawn Base From Name
  (for _index (range 0 (- (Variables|Base|GetShelveSections) 1))
    (for _array_element (Variables|Base|GetSectionBaseArray)
      (bind _output_get (Variables|Base|SetBaseUnitElement _array_element))
      (Variables|Base|SetBaseUnitLocation (Math|Vector|MakeVector (Math|Conversions|ToFloat(Integer) (* _index (Variables|Base|Getsection_offset))) 0.0 0.0))
      (if (Utilities|Enum|Equal(Enum) (Utilities|String|LeftChop (Utilities|GetClassDisplayName _array_element) 2) _baseunit)
        (CallFunction|SpawnBaseElement _baseunit (Variables|Base|Getsection_offset) (Variables|Base|GetBaseUnitLocation) _output_get)))))

(event Custom|SpawnBaseElement
  (params (name :type String) (width_offset :type Integer) (location :type Vector) (base%20actor :type Actor%20Class%20Reference))
  ;[1 1 1] Spawn Section Bases
  (Game|SpawnActorfromClass base%20actor (Math|Transform|MakeTransform location) "Undefined" 0 0))

(fn ConverttoVector
  (params (X :type String) (Y :type String) (Z :type String))
  (return (Math|Vector|MakeVector (Math|Conversions|ToFloat(Integer) X) (Math|Conversions|ToFloat(Integer) Y) (Math|Conversions|ToFloat(Integer) Z))))

(fn BuildBlueprintName
  (params (UPC :type String))
  ;[1 1 1] Build BA String from CSV file
  (Variables|Placeable|SetBA_String (Utilities|String|Append (Variables|Placeable|GetBA_Append) UPC)))

(fn ResetDepthOffset
  (return 0.0))

(fn ResetWidthOffset
  (return 0.0))

(fn SetProductLocation
  (params (x_position :type String) (y_position :type String) (z_position :type String))
  (bind _returnvalue (Utilities|String|LeftChop y_position 2))
  (bind _returnvalue_2 (Utilities|String|LeftChop z_position 2))
  (bind _returnvalue_3 (Utilities|String|LeftChop x_position 2))
  ;[1 1 1] Set Product Location
  (Variables|Placeable|Setx_position (Math|Conversions|ToFloat(Integer) _returnvalue_3))
  (Variables|Placeable|Sety_position (Math|Conversions|ToFloat(Integer) _returnvalue_2))
  (Variables|Placeable|Setz_position (Math|Conversions|ToFloat(Integer) _returnvalue))
  (bind _size (CallFunction|ConverttoVector _returnvalue_3 _returnvalue_2 _returnvalue))
  (Variables|Placeable|Setplaceable_location _size)
  (return))

(fn SetProductOffset
  (params (X%20Offset :type String) (Y%20Offset :type String) (Z%20Offset :type String))
  (bind _output_get (Variables|Placeable|Sety_offset (Math|Conversions|ToFloat(Integer) (Utilities|String|LeftChop X%20Offset 2))))
  (bind _output_get_2 (Variables|Placeable|Setx_offset (Math|Conversions|ToFloat(Integer) (Utilities|String|LeftChop Y%20Offset 2))))
  (bind _output_get_3 (Variables|Placeable|Setz_offset (Math|Conversions|ToFloat(Integer) (Utilities|String|LeftChop Z%20Offset 2)))))

(fn GetMaxDepth)

(fn ShelfConverttoFloat
  (params (data :type String))
  ;[1 1 1] Convert To Float
  (return (Math|Conversions|ToFloat(Integer) (Utilities|String|RightChop (Utilities|String|LeftChop data 3) 2))))

(fn SetShelfYLocation
  (params (Y%20Position :type String))
  ;[1 1 1] Set Shelve Y Position
  (bind _output_get (Variables|Shelves|SetShelve_height (Math|Conversions|ToFloat(Integer) (Utilities|String|LeftChop Y%20Position 2))))
  (return _output_get))

(fn SetShelfXLocation
  (params (X%20Position :type String))
  ;[1 1 1] Set Shelve X Position
  (bind _output_get (Variables|Shelves|SetShelve_height (Math|Conversions|ToFloat(Integer) (Utilities|String|LeftChop X%20Position 2))))
  (return _output_get))

(fn SetShelfSize
  (params (x_position :type String) (y_position :type String) (z_position :type String))
  (bind _returnvalue (Utilities|String|LeftChop z_position 2))
  (bind _returnvalue_2 (Utilities|String|LeftChop y_position 2))
  (bind _returnvalue_3 (Utilities|String|LeftChop x_position 2))
  (bind _returnvalue_4 (Utilities|String|RightChop _returnvalue 3))
  (bind _returnvalue_5 (Utilities|String|RightChop _returnvalue_3 3))
  (bind _returnvalue_6 (Utilities|String|RightChop _returnvalue_2 3))
  ;[1 1 1] Set Shelf Location
  (Variables|Shelves|Setshelf_width (Math|Conversions|ToFloat(Integer) _returnvalue_5))
  (Variables|Shelves|Setshelf_height (Math|Conversions|ToFloat(Integer) _returnvalue_6))
  (Variables|Shelves|Setshelf_depth (Math|Conversions|ToFloat(Integer) _returnvalue_4))
  (bind _size (CallFunction|ConverttoVector _returnvalue_5 _returnvalue_6 _returnvalue_4))
  (Variables|Shelves|Setshelf%20size _size)
  (return))

(fn SetShelfOffsetLocation
  (params (Offset%20Position :type String))
  ;[1 1 1] Set Shelve Offset Position
  (Variables|Shelves|SetSectionShelfOffset (Math|Conversions|ToInteger(Byte) (Utilities|String|RightChop Offset%20Position 2)))
  (return))