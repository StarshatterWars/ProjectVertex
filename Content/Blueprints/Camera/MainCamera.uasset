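; MainCamera is a camera Blueprint that places itself at a preset transform when play begins.
; BeginPlay calls a SetTransform custom event, which teleports the actor without sweeping to the first CameraTransform entry held by VertexInstance.
; It has no active Tick, overlap or construction logic beyond the parent construction call, so this Blueprint's graph does not move it afterwards unless SetTransform is called again.
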(event Custom|Set%20Transform
  ;[1 1 1] Set Transform
  (Transformation|SetActorTransform (Utilities|Array|Get(acopy) (Variables|/Game/Blueprints/Setup/VertexInstance.VertexInstance_C|GetCameraTransform (Variables|Default|GetVertexInstance))) false true))

(event EventBeginPlay
  (|CallParentFunction)
  (CallFunction|SetTransform))

(event Collision|EventActorBeginOverlap
  (params (OtherActor :type Actor%20Object%20Reference))
  (|CallParentFunction OtherActor) ; This node is disabled and will not be called.\nDrag off pins to build functionality.
)

(event EventTick
  (params (DeltaSeconds :type Float%20%28single-precision%29))
  (|CallParentFunction DeltaSeconds) ; This node is disabled and will not be called.\nDrag off pins to build functionality.
)

(fn ConstructionScript
  (|CallParentFunction))