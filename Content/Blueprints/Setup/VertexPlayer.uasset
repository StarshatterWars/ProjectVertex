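; Player pawn that flies the camera for authoring camera keyframes and switching between Editor, Record and Playback modes.
; Movement and look input, gated by flags on the VertexInstance game instance, writes location and rotation back there, while hotkeys toggle movement, recording, preview and display mode.
; Right-click drops a waypoint and timeline entry while moving, and also feeds the pose to any active camera recorder as a keyframe.
; BeginPlay attaches the level's single BP_Gizmo.
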(event EventTick
  (params (DeltaSeconds :type Float%20%28single-precision%29)))

(event EventBeginPlay
  (bind _returnvalue (Game|GetPlayerController 0))
  ;[1 1 1] Setup
  (Utilities|FlowControl|Sequence
    (:then_0
      (bind _asvertex_instance (Utilities|Casting|CastToVertexInstance (Game|GetGameInstance)))
      (Variables|Default|SetAs%20Vertex%20Instance _asvertex_instance)
      (Variables|Default|SetMainCameraTransform (Transformation|GetWorldTransform (Variables|Default|GetMainCamera)))
      (Variables|/Script/Engine.PlayerController|SetbShowMouseCursor _returnvalue true)
      (Input|SetInputModeGameandUI _returnvalue 0 "DoNotLock" true))
    (:then_1
      (bind _outactors (Actor|GetAllActorsOfClass "/Game/RuntimeGizmo/Blueprints/BP_Gizmo.BP_Gizmo_C"))
      (if (!= (Utilities|Array|Length _outactors) 1)
        (Development|PrintString "ERROR: There should be exactly a single instance of BP_Gizmo in the level." true true "(R=1.000000,G=0.000000,B=0.000000,A=1.000000)" 1e+04)
        (else
          (bind _output_get (Variables|Default|SetGizmoRef (Utilities|Array|Get(acopy) _outactors)))
          (Default|AttachGizmo _output_get self))))))

(event Input|AxisEvents|InputAxisHorizontal
  (params (AxisValue :type Float%20%28single-precision%29))
  (bind _as_vertex_instance (Variables|Default|GetAs%20Vertex%20Instance))
  ;[1 1 1] Move Camera Left/ Right
  (if (or (Variables|/Game/Blueprints/Setup/VertexInstance.VertexInstance_C|GetCameraRecordActive _as_vertex_instance) (Variables|/Game/Blueprints/Setup/VertexInstance.VertexInstance_C|GetPlayerMovementActive _as_vertex_instance))
    (Pawn|Input|AddMovementInput (Transformation|GetActorRightVector) (* AxisValue (Variables|/Game/Blueprints/Setup/VertexInstance.VertexInstance_C|GetCameraMovementSpeed _as_vertex_instance)) false)
    (Variables|/Game/Blueprints/Setup/VertexInstance.VertexInstance_C|SetPlayerLocation (Variables|Default|GetAs%20Vertex%20Instance) (Transformation|GetActorLocation))))

(event Input|AxisEvents|InputAxisVertical
  (params (AxisValue :type Float%20%28single-precision%29))
  (bind _as_vertex_instance (Variables|Default|GetAs%20Vertex%20Instance))
  ;[1 1 1] Move Camera Forward/ Back
  (if (or (Variables|/Game/Blueprints/Setup/VertexInstance.VertexInstance_C|GetCameraRecordActive _as_vertex_instance) (Variables|/Game/Blueprints/Setup/VertexInstance.VertexInstance_C|GetPlayerMovementActive _as_vertex_instance))
    (Pawn|Input|AddMovementInput (Transformation|GetActorForwardVector) (* AxisValue (Variables|/Game/Blueprints/Setup/VertexInstance.VertexInstance_C|GetCameraMovementSpeed _as_vertex_instance)) false)
    (Variables|/Game/Blueprints/Setup/VertexInstance.VertexInstance_C|SetPlayerLocation (Variables|Default|GetAs%20Vertex%20Instance) (Transformation|GetActorLocation))))

(event Input|AxisEvents|InputAxisLook
  (params (AxisValue :type Float%20%28single-precision%29))
  (bind _as_vertex_instance (Variables|Default|GetAs%20Vertex%20Instance))
  ;[1 1 1] Camera Look
  (if (or (Variables|/Game/Blueprints/Setup/VertexInstance.VertexInstance_C|GetCameraRecordActive _as_vertex_instance) (Variables|/Game/Blueprints/Setup/VertexInstance.VertexInstance_C|GetPlayerMovementActive _as_vertex_instance))
    (Pawn|Input|AddControllerPitchInput (* AxisValue (Variables|/Game/Blueprints/Setup/VertexInstance.VertexInstance_C|GetCameraMovementSpeed _as_vertex_instance)))
    (Variables|/Game/Blueprints/Setup/VertexInstance.VertexInstance_C|SetPlayerRotation (Variables|Default|GetAs%20Vertex%20Instance) (Transformation|GetActorRotation))))

(event Input|AxisEvents|InputAxisRotate
  (params (AxisValue :type Float%20%28single-precision%29))
  (bind _as_vertex_instance (Variables|Default|GetAs%20Vertex%20Instance))
  ;[1 1 1] Camera Rotate
  (if (or (Variables|/Game/Blueprints/Setup/VertexInstance.VertexInstance_C|GetCameraRecordActive _as_vertex_instance) (Variables|/Game/Blueprints/Setup/VertexInstance.VertexInstance_C|GetPlayerMovementActive _as_vertex_instance))
    (Pawn|Input|AddControllerYawInput (* AxisValue (Variables|/Game/Blueprints/Setup/VertexInstance.VertexInstance_C|GetCameraMovementSpeed _as_vertex_instance)))
    (Variables|/Game/Blueprints/Setup/VertexInstance.VertexInstance_C|SetPlayerRotation (Variables|Default|GetAs%20Vertex%20Instance) (Transformation|GetActorRotation))))

(event Input|KeyboardEvents|C
  (params (Key :type Key%20Structure))
  ;[1 1 1] Keys
  (:Pressed
    (switch Utilities|FlowControl|Switch|SwitchonE_RunMode (Variables|/Game/Blueprints/Setup/VertexInstance.VertexInstance_C|GetDisplayMode (Variables|Default|GetAs%20Vertex%20Instance))
      (:NewEnumerator1
        _)
      (:NewEnumerator2
        _))
    (bind _isa (Utilities|FlowControl|FlipFlop)
      (:A
        (Default|MovePlayer (Variables|Default|GetAs%20Vertex%20Instance)))
      (:B
        (Default|StopPlayer (Variables|Default|GetAs%20Vertex%20Instance))))
    (Variables|/Game/Blueprints/Setup/VertexInstance.VertexInstance_C|SetPlayerMovementActive (Variables|Default|GetAs%20Vertex%20Instance) _isa)))

(event Input|KeyboardEvents|F3
  (params (Key :type Key%20Structure))
  (:Pressed
    (Development|ExecuteConsoleCommand "stat fps" 0)))

(event Input|KeyboardEvents|F12
  (params (Key :type Key%20Structure))
  ;[1 1 1] Keys
  (:Pressed
    (Default|SetCameraRecord (Variables|Default|GetAs%20Vertex%20Instance))))

(event Input|MouseEvents|RightMouseButton
  (params (Key :type Key%20Structure))
  (bind _as_vertex_instance (Variables|Default|GetAs%20Vertex%20Instance))
  (bind _as_vertex_instance_2 (Variables|Default|GetAs%20Vertex%20Instance))
  (bind _playerlocation (Variables|/Game/Blueprints/Setup/VertexInstance.VertexInstance_C|GetPlayerLocation _as_vertex_instance))
  (bind _playerrotation (Variables|/Game/Blueprints/Setup/VertexInstance.VertexInstance_C|GetPlayerRotation _as_vertex_instance))
  ;[1 1 1] Add Keyframe
  (:Pressed
    (Utilities|FlowControl|Sequence
      (:then_0
        (Development|PrintString (Utilities|String|ToString(Vector) _playerlocation))
        (if (Variables|/Game/Blueprints/Setup/VertexInstance.VertexInstance_C|GetPlayerMovementActive (Variables|Default|GetAs%20Vertex%20Instance))
          (Game|SpawnActorfromClass "/Game/UI/WaypointMarker.WaypointMarker_C" (Math|Transform|MakeTransform _playerlocation _playerrotation "1,1,1") "Undefined" 0 0)
          (Utilities|Array|Add (Variables|/Game/Blueprints/Setup/VertexInstance.VertexInstance_C|GetTimelineCameraData (Variables|Default|GetAs%20Vertex%20Instance)) (Utilities|Struct|MakeS_TimelineCameraRecord 0 (Variables|/Game/Blueprints/Setup/VertexInstance.VertexInstance_C|GetActive%20Configuration%20Nr _as_vertex_instance_2) (Variables|/Game/Blueprints/Setup/VertexInstance.VertexInstance_C|GetActive%20Chapter%20Nr _as_vertex_instance_2) (Variables|Default|GetKeyframeNr) (Variables|/Game/Blueprints/Setup/VertexInstance.VertexInstance_C|GetNewCameraKeyframeTime (Variables|Default|GetAs%20Vertex%20Instance)) _playerlocation _playerrotation 0.0))
          (Variables|Default|SetKeyframeNr (+ (Variables|Default|GetKeyframeNr) 1))))
      (:then_1
        ;[1 1 1] Get the Spline to record
        (bind (_isvalid_ _activecamerarecorder) (CallFunction|GetActiveCameraRecorder self))
        (if _isvalid_
          (Transformation|SetActorLocation (Variables|/Game/RuntimeSplineEditor/Cinematic_SplineTool/Cinematic_Spline/Cinematic_Spline_BP.Cinematic_Spline_BP_C|GetCameraActor _activecamerarecorder) _playerlocation false false)
          (Transformation|SetActorRotation (Variables|/Game/RuntimeSplineEditor/Cinematic_SplineTool/Cinematic_Spline/Cinematic_Spline_BP.Cinematic_Spline_BP_C|GetCameraActor _activecamerarecorder) _playerrotation)
          ;;[1 1 1] Apply the new point
          (Default|AddAdditionalKeyframe _activecamerarecorder))))))

(event Input|KeyboardEvents|R
  (params (Key :type Key%20Structure))
  ;[1 1 1] Keys
  (:Pressed
    (switch Utilities|FlowControl|Switch|SwitchonE_RunMode (Variables|/Game/Blueprints/Setup/VertexInstance.VertexInstance_C|GetDisplayMode (Variables|Default|GetAs%20Vertex%20Instance))
      (:NewEnumerator2
        (Utilities|FlowControl|FlipFlop
          (:A
            (Default|TurnonRecording (Variables|Default|GetAs%20Vertex%20Instance)))
          (:B
            (Default|TurnOffRecording (Variables|Default|GetAs%20Vertex%20Instance))))))))

(event Input|KeyboardEvents|Insert
  (params (Key :type Key%20Structure))
  ;[1 1 1] Keys
  (:Pressed
    (bind _isa (Utilities|FlowControl|FlipFlop)
      (:A
        (Default|MovePlayer (Variables|Default|GetAs%20Vertex%20Instance)))
      (:B
        (Default|StopPlayer (Variables|Default|GetAs%20Vertex%20Instance))))
    (Default|SetCameraEditModeon (Variables|Default|GetAs%20Vertex%20Instance) _isa)
    (Variables|/Game/Blueprints/Setup/VertexInstance.VertexInstance_C|SetPlayerMovementActive (Variables|Default|GetAs%20Vertex%20Instance) _isa)))

(event Input|KeyboardEvents|Escape
  (params (Key :type Key%20Structure))
  (:Pressed
    (Game|QuitGame 0 "Quit" false)))

(event Input|KeyboardEvents|B
  (params (Key :type Key%20Structure))
  (bind _as_vertex_instance (Variables|Default|GetAs%20Vertex%20Instance))
  ;[1 1 1] Camera Preview
  (:Pressed
    (Variables|/Game/Blueprints/Setup/VertexInstance.VertexInstance_C|SetPreviewActiveRecordingCamera _as_vertex_instance (not (Variables|/Game/Blueprints/Setup/VertexInstance.VertexInstance_C|GetPreviewActiveRecordingCamera _as_vertex_instance)))))

(event Input|KeyboardEvents|F2
  (params (Key :type Key%20Structure))
  (:Pressed
    (Variables|/Game/Blueprints/Setup/VertexInstance.VertexInstance_C|SetDisplayMode (Variables|Default|GetAs%20Vertex%20Instance) "NewEnumerator0")))

(event Input|KeyboardEvents|F10
  (params (Key :type Key%20Structure))
  (:Pressed
    (Variables|/Game/Blueprints/Setup/VertexInstance.VertexInstance_C|SetDisplayMode (Variables|Default|GetAs%20Vertex%20Instance) "NewEnumerator1")
    (Variables|/Game/Blueprints/Setup/VertexInstance.VertexInstance_C|SetActiveTitleIndex (Variables|Default|GetAs%20Vertex%20Instance) 1)))

(event Input|KeyboardEvents|Up
  (params (Key :type Key%20Structure))
  (bind _returnvalue (Transformation|GetActorLocation))
  ;[1 1 1] Key Up
  (:Pressed
    (if (Variables|/Game/Blueprints/Setup/VertexInstance.VertexInstance_C|GetPlayerMovementActive (Variables|Default|GetAs%20Vertex%20Instance))
      (Transformation|SetActorLocation (Math|Vector|MakeVector (.x _returnvalue) (.y _returnvalue) (+ (.z _returnvalue) (* (Variables|/Game/Blueprints/Setup/VertexInstance.VertexInstance_C|GetCameraMovementSpeed (Variables|Default|GetAs%20Vertex%20Instance)) 1e+01))) false false))))

(event Input|KeyboardEvents|Down
  (params (Key :type Key%20Structure))
  (bind _returnvalue (Transformation|GetActorLocation))
  ;[1 1 1] Key Down
  (:Pressed
    (if (Variables|/Game/Blueprints/Setup/VertexInstance.VertexInstance_C|GetPlayerMovementActive (Variables|Default|GetAs%20Vertex%20Instance))
      (Transformation|SetActorLocation (Math|Vector|MakeVector (.x _returnvalue) (.y _returnvalue) (+ (.z _returnvalue) (* (Variables|/Game/Blueprints/Setup/VertexInstance.VertexInstance_C|GetCameraMovementSpeed (Variables|Default|GetAs%20Vertex%20Instance)) -1e+01))) false false))))

(fn ConstructionScript)