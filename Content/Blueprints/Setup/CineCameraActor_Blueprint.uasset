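; Cine camera actor Blueprint that switches between a top-down edit view and a main view.
; It caches the VertexInstance game instance on BeginPlay and applies the main view.
; Every Tick it polls that instance's EditCameraOn flag and snaps the camera and scene components to one of two transforms stored in its CameraTransform array, with no blending.
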(event Custom|Set%20Main%20Camera
  ;[1 1 1] Set Main Camera
  (Transformation|SetWorldTransform (Variables|CameraActor|GetCameraComponent) (Utilities|Array|Get(acopy) (Variables|/Game/Blueprints/Setup/VertexInstance.VertexInstance_C|GetCameraTransform (Variables|Default|GetVertexInstance)) 1) false false))

(event Custom|Set%20Top%20Down%20Camera
  ;[1 1 1] Set Top Down Camera
  (Transformation|SetWorldTransform (Variables|CameraActor|GetCameraComponent) (Utilities|Array|Get(acopy) (Variables|/Game/Blueprints/Setup/VertexInstance.VertexInstance_C|GetCameraTransform (Variables|Default|GetVertexInstance))) false false))

(event EventBeginPlay
  ;[1 1 1] Event Construct
  (bind _asvertex_instance (Utilities|Casting|CastToVertexInstance (Game|GetGameInstance)))
  (Variables|Default|SetVertexInstance _asvertex_instance)
  (CallFunction|SetMainCamera))

(event EventTick
  (params (DeltaSeconds :type Float%20%28single-precision%29))
  (if (Variables|/Game/Blueprints/Setup/VertexInstance.VertexInstance_C|GetEditCameraOn (Variables|Default|GetVertexInstance))
    (CallFunction|SetTopDownCamera)
    (else
      (CallFunction|SetMainCamera))))

(event Collision|EventActorBeginOverlap
  (params (OtherActor :type Actor%20Object%20Reference)))

(fn ConstructionScript)